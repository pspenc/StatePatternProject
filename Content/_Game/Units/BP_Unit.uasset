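; BP_Unit is a base unit that serves as either the player's character or an enemy that hunts the player.
; When possessed by the first player controller, it hides its overhead health bar, creates a spring arm and camera at runtime, and wakes BP_UnitPlayerController.
; On BeginPlay it binds itself to the health bar widget.
; Each tick, non-player units move toward the player through CurrentState, attacking once within close range.
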(event EventTick
  (params (DeltaSeconds :type Float%20%28single-precision%29))
  (bind _returnvalue (Game|GetPlayerCharacter 0))
  (bind _self self)
  (if (!= (Game|GetPlayerCharacter 0) self)
    (if (> (Transformation|GetDistanceTo _returnvalue _self) 1.5e+02)
      (Class|UnitState|Move (Variables|Default|GetCurrentState) (Math|Vector|GetUnitDirection(Vector) (Transformation|GetActorLocation _self) (Transformation|GetActorLocation _returnvalue)) 1.0)
      (else
        (Class|Unit|Attack)))))

(event Collision|EventActorBeginOverlap
  (params (OtherActor :type Actor%20Object%20Reference)))

(event EventPossessed
  (params (NewController :type Controller%20Object%20Reference))
  (Utilities|FlowControl|Sequence
    (:then_0
      (if (== NewController (Game|GetPlayerController 0))
        (Rendering|SetVisibility (Variables|Default|GetHealthBar) false false)
        (bind _returnvalue (AddComponent|AddSpringArmComponent false))
        (Variables|Default|SetSpringArm _returnvalue)
        (bind _returnvalue_2 (AddComponent|AddCameraComponent false))
        (bind _output_get (Variables|Default|SetCamera _returnvalue_2))
        (Transformation|AttachComponentToComponent _output_get (Variables|Default|GetSpringArm) "None" "SnapToTarget" "SnapToTarget" "SnapToTarget" true)
        (bind _asbp_unit_player_controller (Utilities|Casting|CastToBP_UnitPlayerController (Game|GetPlayerController 0)))
        (Default|WAkeup _asbp_unit_player_controller)))))

(event EventBeginPlay
  (bind _asui_enemy_overhead_health_bar (Utilities|Casting|CastToUI_EnemyOverheadHealthBar (UserInterface|GetUserWidgetObject (Variables|Default|GetHealthBar))))
  (Default|AssignUnit _asui_enemy_overhead_health_bar self))

(fn ConstructionScript)